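; A template actor for a hinged, door-like mesh that swings open away from the player and closes again.
; BeginPlay caches the player character; OpenIt plays a timeline when closed and otherwise reverses it, marking it closed once the reverse finishes.
; On opening, a dot product between the player-to-actor direction and the scene's forward vector picks the swing side, driving mesh yaw toward plus or minus 90 degrees.
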(event `OpenIt`
  (bind _scene (`self.Scene`))
  (if (`self.IsClosed?`)
    (set `self.IsClosed?` false)
    (set `self.DotProduct` (`KismetMathLibrary.Dot_VectorVector` (`KismetMathLibrary.Normal` (- (`SceneComponent.K2_GetComponentLocation` _scene) (`self.K2_GetActorLocation` (`self.PlayerRef`)))) (`SceneComponent.GetForwardVector` _scene)))
    (bind (_direction _alpha) (`Timeline|OpenTL` :!label _label)
      (:`Update`
        (`SceneComponent.K2_SetRelativeRotation` (`self.StaticMesh`) (`KismetMathLibrary.MakeRotator` 0.0 0.0 (`KismetMathLibrary.Lerp` _alpha (`KismetMathLibrary.SelectFloat` 90.0 -90.0 (>= (`self.DotProduct`) 0.0)) _alpha)) false false))
      (:`Finished`
        (switch `ETimelineDirection` _direction
          (:`Backward`
            (set `self.IsClosed?` true)))))
    (else
      (goto _label :!via `Reverse`))))

(event `self.ReceiveBeginPlay`
  (bind _ascharacter (cast `Character` (`GameplayStatics.GetPlayerCharacter` 0)))
  (set `self.PlayerRef` _ascharacter))

(fn `UserConstructionScript`)