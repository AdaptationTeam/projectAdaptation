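; BP_ChildCharacter is a child character Blueprint that adds interact and ball-summoning inputs to its parent.
; Interact scans actors overlapping the capsule and sends InteractionMessage to the first one implementing BPi_Interaction.
; SummonBall spawns a Ball just ahead of the capsule along the follow camera's forward vector, matching the camera's rotation and ignoring collisions at spawn.
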(event `InputAction|Interact`
  (params (Key :type "Key Structure"))
  (:`Pressed`
    (for _array_element (`PrimitiveComponent.GetOverlappingActors` (`self.CapsuleComponent`) null)
      (if (`KismetSystemLibrary.DoesImplementInterface` _array_element "/Game/OurContent/BPi_Interaction.BPi_Interaction_C")
        (message `/Game/OurContent/BPi_Interaction.Interaction` _array_element null)
        (break)))))

(event `InputAction|SummonBall`
  (params (Key :type "Key Structure"))
  (bind _returnvalue (`SceneComponent.K2_GetComponentRotation` (`self.FollowCamera`)))
  (:`Pressed`
    (`|SpawnActorFromClass` "/Game/OurContent/Magic/Ball.Ball_C" (`KismetMathLibrary.MakeTransform` (+ (`SceneComponent.K2_GetComponentLocation` (`self.CapsuleComponent`)) (* (`KismetMathLibrary.Conv_RotatorToVector` _returnvalue) 100.0)) _returnvalue) "AlwaysSpawn" "OverrideRootScale" null null)))

(fn `UserConstructionScript`
  (`parent.UserConstructionScript`))